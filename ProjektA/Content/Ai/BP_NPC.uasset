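; Zombie NPC that melees the player and can be killed through its Hit event.
; While the player overlaps the Cylinder trigger, a delay-driven loop plays the attack animation, subtracts health stored on EeriePlayerController and updates the player's UI.
; Hit lowers NpcHp; at zero it plays death animation and sound, stops the AI brain and disables capsule collision.
; Tick refreshes the widget health bar and rotates it using a look-at toward the camera.
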(event OnComponentBeginOverlap(Cylinder)
  (params (OverlappedComponent :type Primitive%20Component%20Object%20Reference) (OtherActor :type Actor%20Object%20Reference) (OtherComp :type Primitive%20Component%20Object%20Reference) (OtherBodyIndex :type Integer) (bFromSweep :type Boolean) (SweepResult :type Hit%20Result%20Structure%20%28by%20ref%29))
  (if (== OtherActor (Game|GetPlayerCharacter 0))
    (bind _output_get (Variables|Default|SetInArea true))
    (if (and _output_get (> (Variables|/Game/EeriePlayerController.EeriePlayerController_C|GetPlayerHP (Variables|Default|GetPlayerController)) 0.0)) :!label _label
      (Components|Animation|PlayAnimation (Variables|Character|GetMesh) "/Game/Ai/Animations/Zombie_Attack.Zombie_Attack" false)
      (Utilities|FlowControl|Delay 1.0)
      (bind _output_get_2 (Variables|/Game/EeriePlayerController.EeriePlayerController_C|SetPlayerHP (Variables|Default|GetPlayerController) (- (Variables|/Game/EeriePlayerController.EeriePlayerController_C|GetPlayerHP (Variables|Default|GetPlayerController)) 5.0)))
      (Development|PrintString (Utilities|String|ToString(Float) (- (Variables|/Game/EeriePlayerController.EeriePlayerController_C|GetPlayerHP (Variables|Default|GetPlayerController)) 5.0)))
      (Class|BPItoUi|UpdatePlayerHealth(Message) (Variables|Default|GetUser%20Interface) _output_get_2)
      (Utilities|FlowControl|Delay 1.0)
      (goto _label))))

(event OnComponentEndOverlap(Cylinder)
  (params (OverlappedComponent :type Primitive%20Component%20Object%20Reference) (OtherActor :type Actor%20Object%20Reference) (OtherComp :type Primitive%20Component%20Object%20Reference) (OtherBodyIndex :type Integer))
  (Variables|Default|SetInArea false))

(event Custom|Hit
  (params (HitValue :type Float%20%28double-precision%29))
  (CallFunction|DamageUpdate HitValue))

(event EventTick
  (params (DeltaSeconds :type Float%20%28single-precision%29))
  (CallFunction|UpdtateHealthBar))

(event EventBeginPlay
  (bind _aseerie_player_controller (Utilities|Casting|CastToEeriePlayerController (Game|GetPlayerController 0)))
  (bind _output_get (Variables|Default|SetPlayerController _aseerie_player_controller))
  (Variables|Default|SetUser%20Interface (Variables|/Game/EeriePlayerController.EeriePlayerController_C|GetUserInterface _output_get)))

(fn ConstructionScript)

(fn DamageUpdate
  (params (HitValue :type Float%20%28double-precision%29))
  (if (<= (- (Variables|Default|GetNpcHp) HitValue) 0.0)
    (Variables|Default|SetNpcHp 0.0)
    (Components|Animation|PlayAnimation (Variables|Character|GetMesh) "/Game/Ai/Animations/Dying.Dying" false)
    (bind _output_get (Variables|Default|SetAiController (AI|GetAIController self)))
    (AI|Logic|StopLogic (Variables|/Script/AIModule.AIController|GetBrainComponent _output_get) "Dead")
    (Collision|SetCollisionEnabled (Variables|Collision|GetCapsuleComponent) "NoCollision")
    (Audio|PlaySoundatLocation "/Game/Sounds/zombie-death-2-95167.zombie-death-2-95167" (Transformation|GetActorLocation) "0, 0, 0" 1.5 1.0 0.0 0 0 0 0)
    (return)
    (else
      (Variables|Default|SetNpcHp (- (Variables|Default|GetNpcHp) HitValue))
      (return))))

(fn UpdtateHealthBar
  (bind _returnvalue (Game|GetPlayerCameraManager 0))
  (bind _healthbarwidget (Variables|Default|GetHealthBarWidget))
  (bind _returnvalue_2 (Transformation|GetWorldLocation _healthbarwidget))
  (bind _transformcomponent (Variables|/Script/Engine.PlayerCameraManager|GetTransformComponent _returnvalue))
  (bind _returnvalue_3 (Transformation|GetWorldLocation _transformcomponent))
  (bind _returnvalue_4 (Math|Rotator|FindLookatRotation _returnvalue_2 _returnvalue_3))
  (bind _ashealthbar (Utilities|Casting|CastToHealthbar (UserInterface|GetWidget (Variables|Default|GetHealthBarWidget)))
    (:then
      (Progress|SetPercent (Variables|/Game/Ai/Healthbar.Healthbar_C|GetHealthBar _ashealthbar) (/ (Variables|Default|GetNpcHp) 1e+02))
      (Transformation|SetWorldRotation _healthbarwidget (Math|Rotator|MakeRotator (.roll _returnvalue_4) (.pitch _returnvalue_4) 0.0) false false)
      (return))
    (:CastFailed
      (return))))